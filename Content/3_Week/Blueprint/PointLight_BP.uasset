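; PointLight_BP is a point light Blueprint that pulses its brightness over time in a smooth sine wave.
; Every tick, a Math Expression node feeds game time into a sine remapped to the zero-to-one range and scaled by the Intensity variable.
; The Frequency variable sets the pulse rate, and the result drives the PointLightComponent's intensity.
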(event EventTick
  (params (DeltaSeconds :type Float%20%28single-precision%29))
  (Rendering|Components|Light|SetIntensity (Variables|Default|GetPointLightComponent) (|((((sin(2*pi*x*f))*0.500000)+0.500000)*A) (Utilities|Time|GetGameTimeinSeconds) (Variables|Default|GetIntensity) (Math|Trig|GetPI) (Variables|Default|GetFrequency))))

(fn ConstructionScript)