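; Scene component Blueprint that moves its attach parent around a horizontal circle in relative space, despite the "Bobbing" name.
; Each Tick feeds delta time and the Osc accumulator into AccumUpdate to get a phase.
; Cosine and sine math expressions turn that phase, in full turns, into X and Y scaled by Radius.
; The parent's relative location is overwritten without sweep, holding Z at zero.
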(event EventTick
  (params (DeltaSeconds :type Float%20%28single-precision%29))
  (bind _radius (Variables|Default|Getradius))
  (bind _accum_ (Utilities|AccumUpdate (Variables|Default|GetOsc) DeltaSeconds)
    (:Exec<
      (Transformation|SetRelativeLocation (Transformation|GetAttachParent) (Math|Vector|MakeVector (|((cos((x*6.283185)))*r) (.phase (Utilities|Struct|BreakAccum _accum_)) _radius) (|((sin((x*6.283185)))*r) _radius (.phase (Utilities|Struct|BreakAccum _accum_))) 0.0) false false))))